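; Thrown-shield projectile that homes from enemy to enemy, killing each ThirdPersonCharacter it touches.
; A detection-radius overlap queues living characters, and a DoOnce points the ProjectileMovement homing target at the first one's HomingLocation.
; On mesh overlap, the shield ragdolls the victim, clears IsAlive and removes it from the queue.
; It then retargets the next queued character, or destroys itself when none remain.
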(event `self.ShieldDetectionRadius.OnComponentBeginOverlap`
  (params (OverlappedComponent :type "PrimitiveComponent Object Reference") (OtherActor :type "Actor Object Reference") (OtherComp :type "PrimitiveComponent Object Reference") (OtherBodyIndex :type Integer) (bFromSweep :type Boolean) (SweepResult :type "HitResult Structure (by ref)"))
  (bind _entitites_to_destroy (`self.Entitites to Destroy`))
  ;[1 1 1] CollisionEventToDetectEnemies
  (bind _asthird_person_character (cast `/Game/ThirdPersonBP/Blueprints/ThirdPersonCharacter` OtherActor))
  (if (`/Game/ThirdPersonBP/Blueprints/ThirdPersonCharacter.IsAlive` _asthird_person_character)
    (`KismetArrayLibrary.Array_Add` _entitites_to_destroy _asthird_person_character)
    ;[1 1 1] HomeOnInitialTarget
    (`/Engine/EditorBlueprintResources/StandardMacros.DoOnce` false
      (:`Completed`
        (bind _asthird_person_character_2 (cast `/Game/ThirdPersonBP/Blueprints/ThirdPersonCharacter` (`|GetArrayItem` _entitites_to_destroy)))
        (set `ProjectileMovementComponent.HomingTargetComponent` (`/Game/ThirdPersonBP/Blueprints/ThirdPersonCharacter.HomingLocation` _asthird_person_character_2) (`self.ProjectileMovement`))))))

(event `self.ShieldMesh.OnComponentBeginOverlap`
  (params (OverlappedComponent :type "PrimitiveComponent Object Reference") (OtherActor :type "Actor Object Reference") (OtherComp :type "PrimitiveComponent Object Reference") (OtherBodyIndex :type Integer) (bFromSweep :type Boolean) (SweepResult :type "HitResult Structure (by ref)"))
  (bind _entitites_to_destroy (`self.Entitites to Destroy`))
  ;[1 1 1] CollisionEventWithEnemy
  (bind _asthird_person_character (cast `/Game/ThirdPersonBP/Blueprints/ThirdPersonCharacter` OtherActor))
  (`PrimitiveComponent.SetSimulatePhysics` (`Character.Mesh` _asthird_person_character) true)
  (set `/Game/ThirdPersonBP/Blueprints/ThirdPersonCharacter.IsAlive` false _asthird_person_character)
  (`KismetArrayLibrary.Array_RemoveItem` _entitites_to_destroy _asthird_person_character)
  ;[1 1 1] TargetNextEnemyOrDestroyShield
  (if (>= (`KismetArrayLibrary.Array_LastIndex` _entitites_to_destroy) 0)
    (bind _asthird_person_character_2 (cast `/Game/ThirdPersonBP/Blueprints/ThirdPersonCharacter` (`|GetArrayItem` _entitites_to_destroy)))
    (set `ProjectileMovementComponent.HomingTargetComponent` (`/Game/ThirdPersonBP/Blueprints/ThirdPersonCharacter.HomingLocation` _asthird_person_character_2) (`self.ProjectileMovement`))
    (else
      (`self.K2_DestroyActor`))))

(fn `UserConstructionScript`)