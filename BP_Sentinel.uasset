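; BP_Sentinel is a playable pawn with movement, mouse look and an ultimate ability that spawns a shield.
; Axis inputs drive movement relative to control yaw, plus controller yaw and pitch.
; Q calls ProjectileUltimate with Bp_Shield, which spawns the given class at the ShieldSpawnLocation transform.
; The CanShootUltimate flag blocks recasting until a Delay of UltimateCooldown resets it.
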(event `InputAxis|MoveRight`
  (params (AxisValue :type "Float (single-precision)"))
  (bind (_returnvalue_roll _returnvalue_pitch _returnvalue_yaw) (`KismetMathLibrary.BreakRotator` (`self.GetControlRotation`)))
  (`self.AddMovementInput` (`KismetMathLibrary.GetRightVector` (`KismetMathLibrary.MakeRotator` 0.0 0.0 _returnvalue_yaw)) AxisValue))

(event `InputAxis|Turn`
  (params (AxisValue :type "Float (single-precision)"))
  ;[1 1 1] MouseInput
  (`self.AddControllerYawInput` AxisValue))

(event `InputAxis|LookUp`
  (params (AxisValue :type "Float (single-precision)"))
  ;[1 1 1] MouseInput
  (`self.AddControllerPitchInput` AxisValue))

(event `InputAxis|MoveForward`
  (params (AxisValue :type "Float (single-precision)"))
  (bind (_returnvalue_roll _returnvalue_pitch _returnvalue_yaw) (`KismetMathLibrary.BreakRotator` (`self.GetControlRotation`)))
  (`self.AddMovementInput` (`KismetMathLibrary.GetForwardVector` (`KismetMathLibrary.MakeRotator` 0.0 0.0 _returnvalue_yaw)) AxisValue))

(event `ProjectileUltimate`
  (params (ProjectileToSpawn :type "Actor Class Reference"))
  ;[1 1 1] UltimateAbilityEvent
  (if (`self.CanShootUltimate`)
    (set `self.CanShootUltimate` false)
    (`|SpawnActorFromClass` ProjectileToSpawn (`SceneComponent.K2_GetComponentToWorld` (`self.ShieldSpawnLocation`)) "Undefined" "OverrideRootScale" null null)
    (`KismetSystemLibrary.Delay` (`self.UltimateCooldown`))
    (set `self.CanShootUltimate` true)))

(event `Key|Q`
  (params (Key :type "Key Structure"))
  ;[1 1 1] SpawnProjectileUltimate
  (:`Pressed`
    (`self.ProjectileUltimate` "/Game/Blueprints/bp_Shield.bp_Shield_C")))

(fn `UserConstructionScript`)